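; HeldBox is a box the Heavy bot can grab and push, toggled with Space Bar inside its X or Y trigger volumes.
; Grabbing attaches it to the bot, reduces walk speed, locks rotation and plane-constrains movement to the trigger's axis.
; Releasing restores collision and movement, then opens a five-second Tick gate that traces downward to lower the box or snap it onto Steampoint1.
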(event `self.ReceiveBeginPlay`
  ;[1 0.2576 0 1 25] Checks bot base speed as a reference point when releasing the object and reverting the movement speed
  (bind _outactors (`GameplayStatics.GetAllActorsOfClass` "/Game/ThirdPersonBP/Blueprints/Heavy.Heavy_C"))
  (for _array_element _outactors
    (`/Engine/EditorBlueprintResources/StandardMacros.IsValid` _array_element
      (:`Is Valid`
        (set `self.Heavy Base Speed` (`CharacterMovementComponent.MaxWalkSpeed` (`Character.CharacterMovement` _array_element)))
        (break)))))

(event `Key|SpaceBar`
  (params (Key :type "Key Structure"))
  (bind _heavy_bot (`self.Heavy Bot`))
  (bind _object_placeholder (`self.Object Placeholder`))
  (bind _charactermovement (`Character.CharacterMovement` _heavy_bot))
  ;[1 0 0.8002 1 25] Flip flop to push/release the object
  (:`Pressed`
    (if (`/Game/ThirdPersonBP/Blueprints/Heavy.Currently Pushing?` (`self.Heavy Bot`))
      ;[0 0.8187 1 1 25] Changes collision presets to remove any collision issues while pushing
      (`PrimitiveComponent.SetCollisionProfileName` _object_placeholder "BlockAllDynamic" true)
      ;[0 1 0.1607 1 25] Attaches/detaches from component
      (`self.UnlockInputs`)
      (`self.K2_DetachFromActor` "KeepWorld" "KeepWorld" "KeepWorld")
      (set `/Game/ThirdPersonBP/Blueprints/Heavy.Currently Pushing?` false _heavy_bot)
      (set `CharacterMovementComponent.MaxWalkSpeed` (`self.Heavy Base Speed`) _charactermovement)
      (`self.gate`)
      (else
        ;[0 1 0.4682 1 25] Checks if the heavy is currently facing the object
        (if (`self.CheckHeavyRotation`)
          (`PrimitiveComponent.SetCollisionProfileName` _object_placeholder "OverlapAllDynamic" true)
          (`self.LockInputs`)
          (`self.K2_AttachToComponent` (`/Game/ThirdPersonBP/Blueprints/Heavy.Object Transform` (`self.Heavy Bot`)) "None" "SnapToTarget" "SnapToTarget" "KeepWorld")
          (set `/Game/ThirdPersonBP/Blueprints/Heavy.Currently Pushing?` true _heavy_bot)
          (set `CharacterMovementComponent.MaxWalkSpeed` (`self.Heavy Speed Reduction`) _charactermovement))))))

(event `self.ReceiveTick`
  (params (DeltaSeconds :type "Float (single-precision)"))
  (bind _returnvalue (`SceneComponent.K2_GetComponentLocation` (`self.Object Placeholder`)))
  (`/Engine/EditorBlueprintResources/StandardMacros.Gate` true :!label _label
    (:`Exit`
      (bind _outhit (`KismetSystemLibrary.LineTraceSingle` _returnvalue (`KismetMathLibrary.MakeVector` (.x _returnvalue) (.y _returnvalue) (- (.z _returnvalue) 10.0)) "TraceTypeQuery1"))
      (if (`GameplayStatics.BreakHitResult` _outhit)
        (bind _returnvalue_2 (== (`.HitActor` (`GameplayStatics.BreakHitResult` _outhit)) "/Game/Blueprints/Steampoint1.Steampoint1"))
        (if _returnvalue_2
          (`self.K2_SetActorLocation` (select `bool` _returnvalue_2 :`false` (- (`self.K2_GetActorLocation`) (0.0 0.0 1.0)) :`true` (`.ImpactPoint` (`GameplayStatics.BreakHitResult` _outhit))) :!label _label_2))
        (else
          (goto _label_2))))))

(event `gate`
  (`|ExecutionSequence`
    (:`then_0`
      (goto _label :!via `Open`))
    (:`then_1`
      (`KismetSystemLibrary.Delay` 5.0)
      (goto _label :!via `Close`))))

(event `self.Collision Check X.OnComponentBeginOverlap`
  (params (OverlappedComponent :type "PrimitiveComponent Object Reference") (OtherActor :type "Actor Object Reference") (OtherComp :type "PrimitiveComponent Object Reference") (OtherBodyIndex :type Integer) (bFromSweep :type Boolean) (SweepResult :type "HitResult Structure (by ref)"))
  ;[0 0.05359 1 1 25] Checks if the heavy bot is in bounds to start pushing the object, and enables input to allow for pushing script
  (bind _asheavy (cast `/Game/ThirdPersonBP/Blueprints/Heavy` OtherActor))
  (bind _output_get (set `self.Heavy Bot` _asheavy))
  (set `/Game/ThirdPersonBP/Blueprints/Heavy.IsPushable` true _output_get)
  (`self.EnableInput` (`GameplayStatics.GetPlayerController` 0))
  (set `self.ActiveX` true)
  (set `self.ActiveY` false)
  (`KismetSystemLibrary.PrintString` "Locked On Axis Y"))

(event `self.Collision Check Y.OnComponentBeginOverlap`
  (params (OverlappedComponent :type "PrimitiveComponent Object Reference") (OtherActor :type "Actor Object Reference") (OtherComp :type "PrimitiveComponent Object Reference") (OtherBodyIndex :type Integer) (bFromSweep :type Boolean) (SweepResult :type "HitResult Structure (by ref)"))
  ;[0 0.05359 1 1 25] Checks if the heavy bot is in bounds to start pushing the object, and enables input to allow for pushing script
  (bind _asheavy (cast `/Game/ThirdPersonBP/Blueprints/Heavy` OtherActor))
  (bind _output_get (set `self.Heavy Bot` _asheavy))
  (set `/Game/ThirdPersonBP/Blueprints/Heavy.IsPushable` true _output_get)
  (`self.EnableInput` (`GameplayStatics.GetPlayerController` 0))
  (set `self.ActiveY` true)
  (set `self.ActiveX` false)
  (`KismetSystemLibrary.PrintString` "Locked On Axis X"))

(event `self.Collision Check X.OnComponentEndOverlap`
  (params (OverlappedComponent :type "PrimitiveComponent Object Reference") (OtherActor :type "Actor Object Reference") (OtherComp :type "PrimitiveComponent Object Reference") (OtherBodyIndex :type Integer))
  ;[1 0.04843 0.1281 1 25] When the heavy bot leaves these bounds the input is disabled
  (bind _asheavy (cast `/Game/ThirdPersonBP/Blueprints/Heavy` OtherActor))
  (set `/Game/ThirdPersonBP/Blueprints/Heavy.IsPushable` false _asheavy)
  (`self.DisableInput` (`GameplayStatics.GetPlayerController` 0))
  (set `self.ActiveY` false)
  (set `self.ActiveX` false)
  (`KismetSystemLibrary.PrintString` "Unlocked On Axis Y"))

(event `self.Collision Check Y.OnComponentEndOverlap`
  (params (OverlappedComponent :type "PrimitiveComponent Object Reference") (OtherActor :type "Actor Object Reference") (OtherComp :type "PrimitiveComponent Object Reference") (OtherBodyIndex :type Integer))
  ;[1 0.04843 0.1281 1 25] When the heavy bot leaves these bounds the input is disabled
  (bind _asheavy (cast `/Game/ThirdPersonBP/Blueprints/Heavy` OtherActor))
  (set `/Game/ThirdPersonBP/Blueprints/Heavy.IsPushable` false _asheavy)
  (`self.DisableInput` (`GameplayStatics.GetPlayerController` 0))
  (set `self.ActiveX` false)
  (set `self.ActiveY` false)
  (`KismetSystemLibrary.PrintString` "Unlocked On Axis X"))

(fn `LockInputs`
  (bind _charactermovement (`Character.CharacterMovement` (`self.Heavy Bot`)))
  (bind _charactermovement_2 (`Character.CharacterMovement` (`self.Heavy Bot`)))
  ;[0.2793 0 1 1 25] Checks if player is locked to x collision
  (if (`self.ActiveX`)
    ;[0 0.4138 1 1 25] Constrains heavy on to X axis while pushing
    (`MovementComponent.SetPlaneConstraintEnabled` _charactermovement_2 true)
    (`MovementComponent.SetPlaneConstraintAxisSetting` _charactermovement_2 "Y")
    ;[0 1 0.2164 1 25] Locks rotation so box and player stay in place
    (set `CharacterMovementComponent.bOrientRotationToMovement` false (`Character.CharacterMovement` (`self.Heavy Bot`)) :!label _label)
    (else
      ;[1 0 0.04624 1 25] Checks if player is locked to y collision
      (if (`self.ActiveY`)
        ;[1 0.558 0 1 25] Constrains heavy on to Y axis while pushing
        (`MovementComponent.SetPlaneConstraintEnabled` _charactermovement true)
        (`MovementComponent.SetPlaneConstraintAxisSetting` _charactermovement "X")
        (goto _label)))))

(fn `UnlockInputs`
  (bind _charactermovement (`Character.CharacterMovement` (`self.Heavy Bot`)))
  ;[1 0 0.4905 1 25] Resets the plane axis for the player on releasing the object
  (`MovementComponent.SetPlaneConstraintEnabled` _charactermovement false)
  (`MovementComponent.SetPlaneConstraintAxisSetting` _charactermovement "Custom")
  ;[0 1 0.5515 1 25] Gives free rotation back to the heavy
  (set `CharacterMovementComponent.bOrientRotationToMovement` true _charactermovement))

(fn `UserConstructionScript`)