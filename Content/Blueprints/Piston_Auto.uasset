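; Automatic piston Blueprint that endlessly slides its Cube component back and forth between two positions along its relative Y axis.
; On BeginPlay it checks the Opened flag, moves the cube to the matching end with a timed MoveComponentTo, and flips the flag.
; A Delay then wires back to the same check, forming a self-running latent loop with no Tick or external trigger.
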(event `self.ReceiveBeginPlay`
  (bind _cube (`self.Cube`))
  (bind _cube_2 (`self.Cube`))
  (bind (_relativelocation_x _relativelocation_y _relativelocation_z) (`KismetMathLibrary.BreakVector` (`SceneComponent.RelativeLocation` _cube)))
  (bind (_relativelocation_x_2 _relativelocation_y_2 _relativelocation_z_2) (`KismetMathLibrary.BreakVector` (`SceneComponent.RelativeLocation` _cube_2)))
  (if (`self.Opened`) :!label _label
    (`KismetSystemLibrary.MoveComponentTo` _cube (`KismetMathLibrary.MakeVector` _relativelocation_x 240.0 _relativelocation_z) (struct) false false 1.0)
    (set `self.Opened` false)
    (`KismetSystemLibrary.Delay` 1.0)
    (goto _label)
    (else
      (`KismetSystemLibrary.MoveComponentTo` _cube_2 (`KismetMathLibrary.MakeVector` _relativelocation_x_2 720.0 _relativelocation_z_2) (struct) false false 1.0)
      (set `self.Opened` true)
      (`KismetSystemLibrary.Delay` 1.0)
      (goto _label))))

(fn `UserConstructionScript`)