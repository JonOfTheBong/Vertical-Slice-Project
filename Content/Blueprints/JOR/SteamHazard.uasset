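; Steam hazard that periodically lifts a platform and respawns bots that touch its invisible hitbox.
; A looping timer eases the base plate up by a tunable height, holds, then lowers it to its starting Z, pausing once TurnedOff is set.
; Overlaps from Main or Heavy actors call RespawnBot on the ThirdPersonGameMode, independent of the steam state.
; Move targets are relative locations computed from world-space Z.
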(event `self.ReceiveBeginPlay`
  (bind (_returnvalue_x _returnvalue_y _returnvalue_z) (`KismetMathLibrary.BreakVector` (`SceneComponent.K2_GetComponentLocation` (`self.Base_Platform`))))
  ;[0 1 0.7249 1 25] On start set the default location of the base plate
  (set `self.Platform Origin Z` _returnvalue_z)
  ;[0 0.5056 1 1 25] Start the loop of the elevate event
  (bind _returnvalue (`KismetSystemLibrary.K2_SetTimerDelegate` (delegate `Elevate`) (`self.Eruption Time`) true)))

(event `Elevate`
  (bind _base_platform (`self.Base_Platform`))
  (bind (_returnvalue_x _returnvalue_y _returnvalue_z) (`KismetMathLibrary.BreakVector` (`SceneComponent.K2_GetComponentLocation` _base_platform)))
  ;[0.412 0 1 1 25] Check if the steam is turned off
  (if (`self.Turned Off`)
    ;[1 0 0 1 25] If steam turned off stop the event
    (`KismetSystemLibrary.K2_PauseTimerHandle` (stale `self.ReceiveBeginPlay` _returnvalue))
    (else
      ;[1 0.6242 0 1 25] Move plate up to predefined height from developer input
      (`KismetSystemLibrary.MoveComponentTo` _base_platform (`KismetMathLibrary.MakeVector` 0.0 0.0 (+ _returnvalue_z (`self.Elevation Height`))) (struct) true true (`self.Duration Up`))
      ;[1 0.1686 0.8909 1 25] Reset plate to default height
      (`KismetSystemLibrary.Delay` (`self.Hold Time`))
      (`KismetSystemLibrary.MoveComponentTo` (`self.Base_Platform`) (`KismetMathLibrary.MakeVector` 0.0 0.0 (`self.Platform Origin Z`)) (struct) true true (`self.Duration Down`)))))

(event `self.HitDetection.OnComponentBeginOverlap`
  (params (OverlappedComponent :type "PrimitiveComponent Object Reference") (OtherActor :type "Actor Object Reference") (OtherComp :type "PrimitiveComponent Object Reference") (OtherBodyIndex :type Integer) (bFromSweep :type Boolean) (SweepResult :type "HitResult Structure (by ref)"))
  ;[0 1 0.2196 1 25] Checks for bot colliding with the invisible hitbox
  (cast `/Game/ThirdPersonBP/Blueprints/Main` OtherActor
    (:`then`
      _)
    (:`CastFailed`
      (cast `/Game/ThirdPersonBP/Blueprints/Heavy` OtherActor)))
  ;[1 0.0664 0 1 25] Initiates respawn code from the game mode
  (`KismetSystemLibrary.PrintString` "Dead." true true (struct :`R` 1.0 :`A` 1.0))
  (bind _asthird_person_game_mode (cast `/Game/ThirdPersonBP/Blueprints/ThirdPersonGameMode` (`GameplayStatics.GetGameMode`)))
  (`/Game/ThirdPersonBP/Blueprints/ThirdPersonGameMode.RespawnBot` _asthird_person_game_mode))

(fn `UserConstructionScript`)