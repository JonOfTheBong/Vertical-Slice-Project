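; Elevator actor that raises its ElevationPlate while a tagged "Game Object" actor overlaps PlateCollision and lowers it otherwise.
; BeginPlay stores the height limits, mixing world Z for the top with relative Z for the bottom, and starts a looping CheckCollision timer.
; Each tick of that timer scans tagged actors for overlap, then calls an eased MoveComponentTo toward either limit, resetting its DoOnce immediately.
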(event `self.ReceiveBeginPlay`
  (bind _elevation_plate (`self.Elevation Plate`))
  (bind (_returnvalue_x _returnvalue_y _returnvalue_z) (`KismetMathLibrary.BreakVector` (`SceneComponent.K2_GetComponentLocation` (`self.Elevation Plate`))))
  (bind (_relativelocation_x _relativelocation_y _relativelocation_z) (`KismetMathLibrary.BreakVector` (`SceneComponent.RelativeLocation` _elevation_plate)))
  ;[1 0 0.7725 1 25] Sets Origin Point, as well as the minimum and maxmimum heights to clamp, as well as starting the collision check for the elevator
  (`|ExecutionSequence`
    (:`then_0`
      (set `self.Maximum Height X` (+ _returnvalue_z (`self.Maximum Z Height`))))
    (:`then_1`
      (set `self.OriginLocation` (`SceneComponent.K2_GetComponentLocation` _elevation_plate)))
    (:`then_2`
      (set `self.Minimum Height X` _relativelocation_z))
    (:`then_3`
      (`KismetSystemLibrary.K2_SetTimer` null "CheckCollision" 0.25 true))))

(event `CheckCollision`
  ;[0 0.1455 1 1 25] Runs collision check to see if any actors are on the elevator
  (bind _is_colliding_ (`self.CheckOverlappingActors`))
  (`/Engine/EditorBlueprintResources/StandardMacros.DoOnce` false :!label _label
    (:`Completed`
      (if _is_colliding_
        ;[0.07901 1 0 1 25] Moves elevator upwards on collision
        (`KismetSystemLibrary.MoveComponentTo` (`self.Elevation Plate`) (`KismetMathLibrary.MakeVector` 0.0 0.0 (`self.Maximum Height X`)) (struct) true true (`self.Time To Reach Height X`))
        (goto _label :!via `Reset`)
        (else
          ;[1 0 0.04571 1 25] Moves elevator downwards on no collision
          (`KismetSystemLibrary.MoveComponentTo` (`self.Elevation Plate`) (`KismetMathLibrary.MakeVector` 0.0 0.0 (`self.Minimum Height X`)) (struct) true true (`self.Time To Reach Height X`))
          (goto _label :!via `Reset`))))))

(fn `CheckOverlappingActors`
  (returns (`Is Colliding?` :type Boolean))
  (set `self.CollidingActor` null)
  (bind _outactors (`GameplayStatics.GetAllActorsWithTag` "Game Object"))
  (for _array_element _outactors
    (if (`PrimitiveComponent.IsOverlappingActor` (`self.Plate Collision`) _array_element)
      (set `self.CollidingActor` _array_element)
      (break)))
  (`/Engine/EditorBlueprintResources/StandardMacros.IsValid` (`self.CollidingActor`)
    (:`Is Valid`
      (return true))
    (:`Is Not Valid`
      (return false))))

(fn `UserConstructionScript`)