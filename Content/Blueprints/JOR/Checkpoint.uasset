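; Checkpoint actor that saves separate respawn points for the Main robot and Heavy characters.
; Overlapping SpawnCaptureRadius casts the actor to Main or Heavy, then copies the world transform of that character's respawn marker component into the matching respawn transform on ThirdPersonGameMode.
; Separate DoOnce gates let each character capture the checkpoint only once, with a colored on-screen message confirming it.
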(event `self.SpawnCaptureRadius.OnComponentBeginOverlap`
  (params (OverlappedComponent :type "PrimitiveComponent Object Reference") (OtherActor :type "Actor Object Reference") (OtherComp :type "PrimitiveComponent Object Reference") (OtherBodyIndex :type Integer) (bFromSweep :type Boolean) (SweepResult :type "HitResult Structure (by ref)"))
  (bind _returnvalue (`GameplayStatics.GetGameMode`))
  ;[1 0 0.1038 1 25] Checks if actor is either main robot or heavy
  (cast `/Game/ThirdPersonBP/Blueprints/Main` OtherActor
    (:`then`
      ;[0 1 0.4646 1 25] Sets respawn point of checkpoint to mark the respawn point of the character who collided
      (`/Engine/EditorBlueprintResources/StandardMacros.DoOnce` false
        (:`Completed`
          (bind _asthird_person_game_mode (cast `/Game/ThirdPersonBP/Blueprints/ThirdPersonGameMode` _returnvalue))
          (set `/Game/ThirdPersonBP/Blueprints/ThirdPersonGameMode.MainRespawnTransform` (`SceneComponent.K2_GetComponentToWorld` (`self.RespawnTransform (MAIN)`)) _asthird_person_game_mode)
          (`KismetSystemLibrary.PrintString` "Acquired Checkpoint. (MAIN)" true true (struct :`R` 0.612338 :`G` 0.616859 :`B` 1.0 :`A` 1.0)))))
    (:`CastFailed`
      (cast `/Game/ThirdPersonBP/Blueprints/Heavy` OtherActor)
      (`/Engine/EditorBlueprintResources/StandardMacros.DoOnce` false
        (:`Completed`
          (bind _asthird_person_game_mode_2 (cast `/Game/ThirdPersonBP/Blueprints/ThirdPersonGameMode` _returnvalue))
          (set `/Game/ThirdPersonBP/Blueprints/ThirdPersonGameMode.HeavyRespawnTransform` (`SceneComponent.K2_GetComponentToWorld` (`self.RespawnTransform (HEAVY)`)) _asthird_person_game_mode_2)
          (`KismetSystemLibrary.PrintString` "Acquired Checkpoint. (HEAVY)" true true (struct :`R` 1.0 :`G` 0.969604 :`B` 0.59549 :`A` 1.0)))))))

(fn `UserConstructionScript`)