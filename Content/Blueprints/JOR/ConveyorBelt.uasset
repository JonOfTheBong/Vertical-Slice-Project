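; Conveyor belt actor that carries actors overlapping it along the belt's facing direction, forward or reversed.
; Every Tick, it offsets each actor overlapping MovementCollision by ForcebackSpeed scaled by delta time, skipping those tagged "Stationary".
; GetDirectionalVector derives the direction from BeltMesh's forward vector, negated when MovingForward is false.
; Offsets are applied without sweep, so moved actors are not stopped by blocking geometry.
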(event `self.ReceiveTick`
  (params (DeltaSeconds :type "Float (single-precision)"))
  ;[0 1 0.471 1 25] Each tick multiply preset movement speed with the current time
  ;[1 0 0.08073 1 25] Checks direction boolean to provide forward or reverse vector
  (bind _output_vector (`self.GetDirectionalVector`))
  (for _array_element (`PrimitiveComponent.GetOverlappingActors` (`self.Movement Collision`) null)
    (if (not (`self.ActorHasTag` _array_element "Stationary"))
      ;[0.6395 0.2393 1 1 25] For each actor which collides with the belt, they are moved based on the speed and direction of the belt.
      (`self.K2_AddActorWorldOffset` _array_element (* (* DeltaSeconds (`self.ForcebackSpeed`)) _output_vector) false false))))

(fn `GetDirectionalVector`
  (returns (`Output Vector` :type "Vector Structure"))
  (if (`self.MovingForward?`)
    (return (`KismetMathLibrary.GetForwardVector` (`SceneComponent.K2_GetComponentRotation` (`self.BeltMesh`))))
    (else
      (return (* (`KismetMathLibrary.GetForwardVector` (`SceneComponent.K2_GetComponentRotation` (`self.BeltMesh`))) -1.0)))))

(fn `UserConstructionScript`)