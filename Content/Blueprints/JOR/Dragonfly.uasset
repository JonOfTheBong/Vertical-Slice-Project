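; Dragonfly companion actor that follows the player's controlled Main or Heavy pawn and performs an idle flight when that pawn stands still.
; Each tick it reads the pawn's follow point and idle spline, then VInterps its location toward that point.
; When the pawn is stationary and the dragonfly within a per-pawn range, a retriggerable delay starts a timeline moving it along that pawn's spline.
; Movement or leaving range interrupts the idle path.
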(event `self.ReceiveBeginPlay`)

(event `self.ReceiveTick`
  (params (DeltaSeconds :type "Float (single-precision)"))
  (`|ExecutionSequence`
    (:`then_0`
      (set `self.Delta Seconds` DeltaSeconds))
    (:`then_1`
      (`self.Dragonfly Movement`))))

(event `Dragonfly Movement`
  (bind _dragonflyfollowtransform_location (`KismetMathLibrary.BreakTransform` (`self.DragonflyFollowTransform`)))
  (`|ExecutionSequence` :!label _label
    (:`then_0`
      (`self.GetDragonflyTransform`))
    (:`then_1`
      (bind _moving_ (`self.CheckIfTargetMoving`))
      (bind _inrange_ (`self.CheckDistanceToX`))
      (bind _output_get (set `self.InstanceMoving?` (and _inrange_ (not _moving_))))
      (if _output_get
        (`/Engine/EditorBlueprintResources/StandardMacros.DoOnce` false :!label _label_2
          (:`Completed`
            (`KismetSystemLibrary.RetriggerableDelay` (`self.UntilIdleTime`))
            (if (`self.InstanceMoving?`)
              (`KismetSystemLibrary.PrintString` "Initiate Idle Movement" true true (struct :`G` 1.0 :`B` 0.019088 :`A` 1.0))
              (`self.Move On Idle`)
              (else
                (goto _label_2 :!via `Reset`)))))
        (else
          (`KismetSystemLibrary.PrintString` "Stop Idle Movement" true true (struct :`R` 1.0 :`B` 0.037924 :`A` 1.0))
          (goto _label_2 :!via `Reset`))))
    (:`then_2`
      (`self.K2_SetActorTransform` (`KismetMathLibrary.MakeTransform` (`KismetMathLibrary.VInterpTo` (`self.K2_GetActorLocation`) _dragonflyfollowtransform_location (`self.Delta Seconds`) (`self.FollowTime`)))))))

(event `Move On Idle`
  (bind _flyidlepathmain (`self.FlyIdlePathMAIN`))
  (bind _flyidlepathheavy (`self.FlyIdlePathHEAVY`))
  (bind _returnvalue (`Controller.K2_GetPawn` (`GameplayStatics.GetPlayerController` 0)))
  (cast `/Game/ThirdPersonBP/Blueprints/Main` _returnvalue
    (:`then`
      (`TimelineComponent.SetPlayRate` (`self.Movement Timeline (MAIN)`) (/ 1.0 (`self.IdleCompletionTimeMAIN`)))
      (bind (_direction _movement_speed) (`Timeline|Movement Timeline (MAIN)` :!label _label_3)
        (:`Update`
          (if (`self.InstanceMoving?`)
            (bind _returnvalue_2 (`KismetMathLibrary.Lerp` 0.0 (`SplineComponent.GetSplineLength` (`self.FlyIdlePathMAIN`)) _movement_speed))
            (`self.K2_SetActorTransform` (`KismetMathLibrary.MakeTransform` (`SplineComponent.GetLocationAtDistanceAlongSpline` _flyidlepathmain _returnvalue_2 "World") (`SplineComponent.GetRotationAtDistanceAlongSpline` _flyidlepathmain _returnvalue_2 "World")))
            (else
              (`|ExecutionSequence` :!label _label_4
                (:`then_0`
                  (goto _label_3 :!via `Stop`))
                (:`then_1`
                  (goto _label))
                (:`then_2`
                  (bind (_direction_2 _movement_speed_2) (`Timeline|Movement Timeline (HEAVY)` :!via `Stop` :!label _label_5)
                    (:`Update`
                      (if (`self.InstanceMoving?`)
                        (bind _returnvalue_3 (`KismetMathLibrary.Lerp` 0.0 (`SplineComponent.GetSplineLength` (`self.FlyIdlePathHEAVY`)) _movement_speed_2))
                        (`self.K2_SetActorTransform` (`KismetMathLibrary.MakeTransform` (`SplineComponent.GetLocationAtDistanceAlongSpline` _flyidlepathheavy _returnvalue_3 "World") (`SplineComponent.GetRotationAtDistanceAlongSpline` _flyidlepathheavy _returnvalue_3 "World")))
                        (else
                          (goto _label_4))))))))))))
    (:`CastFailed`
      (cast `/Game/ThirdPersonBP/Blueprints/Heavy` _returnvalue)
      (`TimelineComponent.SetPlayRate` (`self.Movement Timeline (HEAVY)`) (/ 1.0 (`self.IdleCompletionTimeHEAVY`)))
      (goto _label_5))))

(fn `CheckDistanceToX`
  (returns (`InRange?` :type Boolean))
  (bind _returnvalue (`Controller.K2_GetPawn` (`GameplayStatics.GetPlayerController` 0)))
  (bind _asmain (cast `/Game/ThirdPersonBP/Blueprints/Main` _returnvalue)
    (:`then`
      (if (>= (`KismetMathLibrary.Vector_Distance` (`SceneComponent.K2_GetComponentLocation` (`/Game/ThirdPersonBP/Blueprints/Main.Dragonfly Follow Transform` _asmain)) (`self.K2_GetActorLocation`)) 100.0)
        (`KismetSystemLibrary.PrintString` "Dragonfly is not in Range" false true (struct :`R` 1.0 :`G` 0.007126 :`A` 1.0))
        (return false)
        (else
          (`KismetSystemLibrary.PrintString` "Dragonfly is in Range" false true (struct :`G` 1.0 :`B` 0.25 :`A` 1.0))
          (return true))))
    (:`CastFailed`
      (bind _asheavy (cast `/Game/ThirdPersonBP/Blueprints/Heavy` _returnvalue))
      (if (>= (`KismetMathLibrary.Vector_Distance` (`SceneComponent.K2_GetComponentLocation` (`/Game/ThirdPersonBP/Blueprints/Heavy.DragonflyFollow` _asheavy)) (`self.K2_GetActorLocation`)) 500.0)
        (`KismetSystemLibrary.PrintString` "Dragonfly is not in Range" true true (struct :`R` 1.0 :`G` 0.007126 :`A` 1.0))
        (return false)
        (else
          (`KismetSystemLibrary.PrintString` "Dragonfly is in Range" true true (struct :`G` 1.0 :`B` 0.25 :`A` 1.0))
          (return true))))))

(fn `CheckIfTargetMoving`
  (returns (`Moving?` :type Boolean))
  (bind _returnvalue (`Controller.K2_GetPawn` (`GameplayStatics.GetPlayerController` 0)))
  (bind _asmain (cast `/Game/ThirdPersonBP/Blueprints/Main` _returnvalue)
    (:`then`
      (if (> (`KismetMathLibrary.VSize` (`MovementComponent.Velocity` (`Character.CharacterMovement` _asmain))) 0.0)
        (`KismetSystemLibrary.PrintString` "Target is moving" false true (struct :`R` 1.0 :`B` 0.03671 :`A` 1.0))
        (return true)
        (else
          (`KismetSystemLibrary.PrintString` "Target is not moving" false true (struct :`G` 1.0 :`B` 0.148475 :`A` 1.0))
          (return false))))
    (:`CastFailed`
      (bind _asheavy (cast `/Game/ThirdPersonBP/Blueprints/Heavy` _returnvalue))
      (if (> (`KismetMathLibrary.VSize` (`MovementComponent.Velocity` (`Character.CharacterMovement` _asheavy))) 0.0)
        (`KismetSystemLibrary.PrintString` "Target is moving" true true (struct :`R` 1.0 :`B` 0.03671 :`A` 1.0))
        (return true)
        (else
          (`KismetSystemLibrary.PrintString` "Target is not moving" true true (struct :`G` 1.0 :`B` 0.148475 :`A` 1.0))
          (return false))))))

(fn `GetDragonflyTransform`
  (bind _returnvalue (`Controller.K2_GetPawn` (`GameplayStatics.GetPlayerController` 0)))
  (bind _asmain (cast `/Game/ThirdPersonBP/Blueprints/Main` _returnvalue)
    (:`then`
      (set `self.DragonflyFollowTransform` (`SceneComponent.K2_GetComponentToWorld` (`/Game/ThirdPersonBP/Blueprints/Main.Dragonfly Follow Transform` _asmain)))
      (set `self.FlyIdlePathMAIN` (`/Game/ThirdPersonBP/Blueprints/Main.Dragonfly Idle Path` _asmain)))
    (:`CastFailed`
      (bind _asheavy (cast `/Game/ThirdPersonBP/Blueprints/Heavy` _returnvalue))
      (set `self.DragonflyFollowTransform` (`SceneComponent.K2_GetComponentToWorld` (`/Game/ThirdPersonBP/Blueprints/Heavy.DragonflyFollow` _asheavy)))
      (set `self.FlyIdlePathHEAVY` (`/Game/ThirdPersonBP/Blueprints/Heavy.DragonflyIdleRoute` _asheavy)))))

(fn `UserConstructionScript`)