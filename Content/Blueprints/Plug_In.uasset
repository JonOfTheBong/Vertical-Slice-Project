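; Plug-in interaction actor with a rotating plane that lets the Main character use a battery, while Heavy only gets a refusal message.
; Box overlap by Main or Heavy toggles input for Interact, which runs a macro switching on Number.
; In the "Power on" case, a matching battery makes Main walk to the Arrow once via MoveComponentTo, restores its AnimBlueprint, then destroys the actor.
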(event `self.ReceiveBeginPlay`
  (`MovementComponent.SetUpdatedComponent` (`self.RotatingMovement`) (`self.Plane`)))

(event `InputAction|Interact`
  (params (Key :type "Key Structure"))
  (:`Pressed`
    (bind _asmain (cast `/Game/ThirdPersonBP/Blueprints/Main` (`GameplayStatics.GetPlayerCharacter` 0))
      (:`then`
        (`self.NewMacro` _asmain _asmain :!label _label))
      (:`CastFailed`
        (goto _label :!via `OnCastFail`)))))

(event `self.Box.OnComponentBeginOverlap`
  (params (OverlappedComponent :type "PrimitiveComponent Object Reference") (OtherActor :type "Actor Object Reference") (OtherComp :type "PrimitiveComponent Object Reference") (OtherBodyIndex :type Integer) (bFromSweep :type Boolean) (SweepResult :type "HitResult Structure (by ref)"))
  (cast `/Game/ThirdPersonBP/Blueprints/Main` OtherActor
    (:`then`
      _)
    (:`CastFailed`
      (cast `/Game/ThirdPersonBP/Blueprints/Heavy` OtherActor)))
  (`self.EnableInput` (`GameplayStatics.GetPlayerController` 0)))

(event `self.Box.OnComponentEndOverlap`
  (params (OverlappedComponent :type "PrimitiveComponent Object Reference") (OtherActor :type "Actor Object Reference") (OtherComp :type "PrimitiveComponent Object Reference") (OtherBodyIndex :type Integer))
  (cast `/Game/ThirdPersonBP/Blueprints/Main` OtherActor
    (:`then`
      _)
    (:`CastFailed`
      (cast `/Game/ThirdPersonBP/Blueprints/Heavy` OtherActor)))
  (`self.DisableInput` (`GameplayStatics.GetPlayerController` 0)))

(fn `UserConstructionScript`)