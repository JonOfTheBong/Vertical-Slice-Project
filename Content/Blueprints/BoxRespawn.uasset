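; BoxRespawn is an interactable actor that replaces a physics box and has a pair of panels that open for it.
; Interact destroys the boxes in its Target array, spawns a new PhysicsBox at the Arrow's transform and stores it as the sole entry.
; A PhysicsBox entering the Box trigger plays the Open timeline through an unreset DoOnce to slide both panels, and leaving reverses it.
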(event `/Game/Blueprints/Interact.Interact`
  (bind _target (`self.Target`))
  (bind (_returnvalue_location _returnvalue_rotation) (`KismetMathLibrary.BreakTransform` (`SceneComponent.K2_GetComponentToWorld` (`self.Arrow`))))
  (for _array_element (`self.Target`)
    (`/Engine/EditorBlueprintResources/StandardMacros.IsValid` _array_element
      (:`Is Valid`
        (`self.K2_DestroyActor` _array_element))))
  (bind _returnvalue (`|SpawnActorFromClass` "/Game/Blueprints/PhysicsBox.PhysicsBox_C" (`KismetMathLibrary.MakeTransform` _returnvalue_location _returnvalue_rotation) "Undefined" "OverrideRootScale" null null))
  (`KismetArrayLibrary.Array_Clear` _target)
  (`KismetArrayLibrary.Array_Add` _target _returnvalue))

(event `self.Box.OnComponentBeginOverlap`
  (params (OverlappedComponent :type "PrimitiveComponent Object Reference") (OtherActor :type "Actor Object Reference") (OtherComp :type "PrimitiveComponent Object Reference") (OtherBodyIndex :type Integer) (bFromSweep :type Boolean) (SweepResult :type "HitResult Structure (by ref)"))
  (cast `/Game/Blueprints/PhysicsBox` OtherActor)
  (`/Engine/EditorBlueprintResources/StandardMacros.DoOnce` false
    (:`Completed`
      (bind (_direction _newtrack_0 _newtrack_1) (`Timeline|Open` :!label _label)
        (:`Update`
          (`SceneComponent.K2_SetRelativeLocation` (`self.L Panel`) _newtrack_0 false false)
          (`SceneComponent.K2_SetRelativeLocation` (`self.R Panel`) _newtrack_1 false false)
          (`KismetSystemLibrary.Delay` 3.0))))))

(event `self.Box.OnComponentEndOverlap`
  (params (OverlappedComponent :type "PrimitiveComponent Object Reference") (OtherActor :type "Actor Object Reference") (OtherComp :type "PrimitiveComponent Object Reference") (OtherBodyIndex :type Integer))
  (cast `/Game/Blueprints/PhysicsBox` OtherActor)
  (goto _label :!via `Reverse`))

(fn `UserConstructionScript`)