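; Battery actor with two box components, XBox and YBox, whose physics simulation responds to overlaps with Heavy actors.
; Each box starts simulating physics when a Heavy begins overlapping it.
; When the overlap ends, XBox stops simulating, while YBox sets simulation to true again, so nothing in this graph turns its physics off.
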(event `self.XBox.OnComponentBeginOverlap`
  (params (OverlappedComponent :type "PrimitiveComponent Object Reference") (OtherActor :type "Actor Object Reference") (OtherComp :type "PrimitiveComponent Object Reference") (OtherBodyIndex :type Integer) (bFromSweep :type Boolean) (SweepResult :type "HitResult Structure (by ref)"))
  (cast `/Game/ThirdPersonBP/Blueprints/Heavy` OtherActor)
  (`PrimitiveComponent.SetSimulatePhysics` (`self.XBox`) true))

(event `self.XBox.OnComponentEndOverlap`
  (params (OverlappedComponent :type "PrimitiveComponent Object Reference") (OtherActor :type "Actor Object Reference") (OtherComp :type "PrimitiveComponent Object Reference") (OtherBodyIndex :type Integer))
  (cast `/Game/ThirdPersonBP/Blueprints/Heavy` OtherActor)
  (`PrimitiveComponent.SetSimulatePhysics` (`self.XBox`) false))

(event `self.YBox.OnComponentBeginOverlap`
  (params (OverlappedComponent :type "PrimitiveComponent Object Reference") (OtherActor :type "Actor Object Reference") (OtherComp :type "PrimitiveComponent Object Reference") (OtherBodyIndex :type Integer) (bFromSweep :type Boolean) (SweepResult :type "HitResult Structure (by ref)"))
  (cast `/Game/ThirdPersonBP/Blueprints/Heavy` OtherActor)
  (`PrimitiveComponent.SetSimulatePhysics` (`self.YBox`) true))

(event `self.YBox.OnComponentEndOverlap`
  (params (OverlappedComponent :type "PrimitiveComponent Object Reference") (OtherActor :type "Actor Object Reference") (OtherComp :type "PrimitiveComponent Object Reference") (OtherBodyIndex :type Integer))
  (cast `/Game/ThirdPersonBP/Blueprints/Heavy` OtherActor)
  (`PrimitiveComponent.SetSimulatePhysics` (`self.YBox`) true))

(fn `UserConstructionScript`)