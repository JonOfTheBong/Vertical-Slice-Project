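; Steam pressure plate puzzle actor whose Cylinder sinks under a "Weighted" actor and returns when the weight leaves.
; Overlaps add or remove its ID in the shared Heavy actor's list, then broadcast RiseUp or FallDown to every Steampoint1.
; A plate rises higher while its partner's ID is listed; both IDs together hide SteamExplosion cubes and activate their Niagara effects.
; Two mutually resetting DoOnce gates alternate press and release.
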(event `self.ReceiveBeginPlay`
  (bind _outactors (`GameplayStatics.GetAllActorsOfClass` "/Game/ThirdPersonBP/Blueprints/Heavy.Heavy_C"))
  (set `self.Heavy` (`|GetArrayItem` _outactors)))

(event `FallDown`
  (bind _pressurebuiltnum (`/Game/ThirdPersonBP/Blueprints/Heavy.PressureBuiltNum` (`self.Heavy`)))
  (if (not (and (`KismetArrayLibrary.Array_Contains` _pressurebuiltnum (`self.OtherPressure`)) (`KismetArrayLibrary.Array_Contains` _pressurebuiltnum (`self.PressureBuilt`))))
    (if (not (`KismetArrayLibrary.Array_Contains` (`/Game/ThirdPersonBP/Blueprints/Heavy.PressureBuiltNum` (`self.Heavy`)) (`self.OtherPressure`)))
      (`KismetSystemLibrary.MoveComponentTo` (`self.Cylinder`) (0.0 0.0 180.0) (struct) false false 1.0))))

(event `Rise up`
  (bind _pressurebuiltnum (`/Game/ThirdPersonBP/Blueprints/Heavy.PressureBuiltNum` (`self.Heavy`)))
  (if (not (and (`KismetArrayLibrary.Array_Contains` _pressurebuiltnum (`self.OtherPressure`)) (`KismetArrayLibrary.Array_Contains` _pressurebuiltnum (`self.PressureBuilt`))))
    (if (`KismetArrayLibrary.Array_Contains` (`/Game/ThirdPersonBP/Blueprints/Heavy.PressureBuiltNum` (`self.Heavy`)) (`self.OtherPressure`))
      (`KismetSystemLibrary.MoveComponentTo` (`self.Cylinder`) (0.0 0.0 360.0) (struct) false false 1.0))
    (else
      (`KismetSystemLibrary.PrintString` "big boom")
      (bind _outactors (`GameplayStatics.GetAllActorsOfClass` "/Game/Blueprints/SteamExplosion.SteamExplosion_C"))
      (for _array_element _outactors
        (`SceneComponent.SetVisibility` (`/Game/Blueprints/SteamExplosion.Cube` _array_element) false false)
        (`ActorComponent.Activate` (`self.GetComponentByClass` _array_element "/Script/Niagara.NiagaraComponent") false)))))

(event `self.Box.OnComponentBeginOverlap`
  (params (OverlappedComponent :type "PrimitiveComponent Object Reference") (OtherActor :type "Actor Object Reference") (OtherComp :type "PrimitiveComponent Object Reference") (OtherBodyIndex :type Integer) (bFromSweep :type Boolean) (SweepResult :type "HitResult Structure (by ref)"))
  (if (`self.ActorHasTag` OtherActor "Weighted")
    (`/Engine/EditorBlueprintResources/StandardMacros.DoOnce` false :!label _label
      (:`Completed`
        (`KismetArrayLibrary.Array_Add` (`/Game/ThirdPersonBP/Blueprints/Heavy.PressureBuiltNum` (`self.Heavy`)) (`self.PressureBuilt`))
        (`KismetSystemLibrary.MoveComponentTo` (`self.Cylinder`) (0.0 0.0 0.0) (struct) true true 1.0)
        (`self.Reset Up`)
        (bind _outactors (`GameplayStatics.GetAllActorsOfClass` "Steampoint1_C"))
        (for _array_element _outactors
          (`self.Rise up` _array_element))))))

(event `Reset Down`
  (goto _label :!via `Reset`))

(event `self.Box.OnComponentEndOverlap`
  (params (OverlappedComponent :type "PrimitiveComponent Object Reference") (OtherActor :type "Actor Object Reference") (OtherComp :type "PrimitiveComponent Object Reference") (OtherBodyIndex :type Integer))
  (if (`self.ActorHasTag` OtherActor "Weighted")
    (`/Engine/EditorBlueprintResources/StandardMacros.DoOnce` false :!label _label_2
      (:`Completed`
        (`KismetArrayLibrary.Array_RemoveItem` (`/Game/ThirdPersonBP/Blueprints/Heavy.PressureBuiltNum` (`self.Heavy`)) (`self.PressureBuilt`))
        (`KismetSystemLibrary.MoveComponentTo` (`self.Cylinder`) (0.0 0.0 180.0) (struct) true true 0.5)
        (`self.Reset Down`)
        (bind _outactors (`GameplayStatics.GetAllActorsOfClass` "Steampoint1_C"))
        (for _array_element _outactors
          (`self.FallDown` _array_element))))))

(event `Reset Up`
  (goto _label_2 :!via `Reset`))

(fn `UserConstructionScript`)