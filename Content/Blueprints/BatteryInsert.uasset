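; BatteryInsert is a battery socket actor that snaps a Battery into place and registers it with the Main actor.
; The first Battery to overlap its Box has physics disabled and is eased toward the Box location and socket Cube rotation, using world values as relative targets.
; As the move starts, the socket adds its BattNum to the Battery collection on every Main actor found in the level.
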(event `self.Box.OnComponentBeginOverlap`
  (params (OverlappedComponent :type "PrimitiveComponent Object Reference") (OtherActor :type "Actor Object Reference") (OtherComp :type "PrimitiveComponent Object Reference") (OtherBodyIndex :type Integer) (bFromSweep :type Boolean) (SweepResult :type "HitResult Structure (by ref)"))
  (bind _asbattery (cast `/Game/Blueprints/Battery` OtherActor))
  (`/Engine/EditorBlueprintResources/StandardMacros.DoOnce` false
    (:`Completed`
      (bind _cube (`/Game/Blueprints/Battery.Cube` _asbattery))
      (`PrimitiveComponent.SetSimulatePhysics` _cube false)
      (`KismetSystemLibrary.MoveComponentTo` _cube (`SceneComponent.K2_GetComponentLocation` (`self.Box`)) (`SceneComponent.K2_GetComponentRotation` (`self.Cube`)) false false 1.0)
      (bind _outactors (`GameplayStatics.GetAllActorsOfClass` "/Game/ThirdPersonBP/Blueprints/Main.Main_C"))
      (for _array_element _outactors
        (`KismetArrayLibrary.Array_Add` (`/Game/ThirdPersonBP/Blueprints/Main.Battery` _array_element) (`self.BattNum`))))))

(fn `UserConstructionScript`)