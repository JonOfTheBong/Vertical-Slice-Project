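; Box spawner actor that keeps dropping WeightedCube actors into the level from three arrow-marked spawn points.
; On BeginPlay, a random looping MultiGate picks one of the arrows and spawns a cube at its location and rotation.
; Each scale axis is randomized independently between the arrow's scale and a fixed upper limit.
; A delay then re-enters the gate, forming an endless timed spawn loop.
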(event `self.ReceiveBeginPlay`
  (bind _returnvalue (`SceneComponent.K2_GetComponentToWorld` (`self.Arrow`)))
  (bind _returnvalue_2 (`SceneComponent.K2_GetComponentToWorld` (`self.Arrow2`)))
  (bind _returnvalue_3 (`SceneComponent.K2_GetComponentToWorld` (`self.Arrow1`)))
  (`|MultiGate` true true 0 :!label _label
    (:`Out 0`
      (`|SpawnActorFromClass` "/Game/Blueprints/WeightedCube.WeightedCube_C" (`KismetMathLibrary.MakeTransform` (.location _returnvalue) (.rotation _returnvalue) (`KismetMathLibrary.MakeVector` (`KismetMathLibrary.RandomFloatInRange` (.x (.scale _returnvalue)) 2.0) (`KismetMathLibrary.RandomFloatInRange` (.y (.scale _returnvalue)) 2.0) (`KismetMathLibrary.RandomFloatInRange` (.z (.scale _returnvalue)) 2.0))) "Undefined" "OverrideRootScale" null null)
      (`KismetSystemLibrary.Delay` 3.0)
      (goto _label))
    (:`Out 1`
      (`|SpawnActorFromClass` "/Game/Blueprints/WeightedCube.WeightedCube_C" (`KismetMathLibrary.MakeTransform` (.location _returnvalue_2) (.rotation _returnvalue_2) (`KismetMathLibrary.MakeVector` (`KismetMathLibrary.RandomFloatInRange` (.x (.scale _returnvalue_2)) 2.0) (`KismetMathLibrary.RandomFloatInRange` (.y (.scale _returnvalue_2)) 2.0) (`KismetMathLibrary.RandomFloatInRange` (.z (.scale _returnvalue_2)) 2.0))) "Undefined" "OverrideRootScale" null null)
      (`KismetSystemLibrary.Delay` 3.0)
      (goto _label))
    (:`Out 2`
      (`|SpawnActorFromClass` "/Game/Blueprints/WeightedCube.WeightedCube_C" (`KismetMathLibrary.MakeTransform` (.location _returnvalue_3) (.rotation _returnvalue_3) (`KismetMathLibrary.MakeVector` (`KismetMathLibrary.RandomFloatInRange` (.x (.scale _returnvalue_3)) 2.0) (`KismetMathLibrary.RandomFloatInRange` (.y (.scale _returnvalue_3)) 2.0) (`KismetMathLibrary.RandomFloatInRange` (.z (.scale _returnvalue_3)) 2.0))) "Undefined" "OverrideRootScale" null null)
      (`KismetSystemLibrary.Delay` 3.0)
      (goto _label))))

(fn `UserConstructionScript`)