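; Test actor for an object the Heavy bot can push along a locked X or Y axis, apparently unfinished.
; BeginPlay caches the first valid Heavy's MaxWalkSpeed as a base speed for restoring movement on release.
; The overlap logic toggling pushability, input, axis flags and physics is disconnected from its empty CollisionCheckX/Y events.
; CheckHeavyRotation holds only an unused yaw-range check for the bot facing the object.
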(event `self.ReceiveBeginPlay`
  ;[1 0.2576 0 1 25] Checks bot base speed as a reference point when releasing the object and reverting the movement speed
  (bind _outactors (`GameplayStatics.GetAllActorsOfClass` "/Game/ThirdPersonBP/Blueprints/Heavy.Heavy_C"))
  (for _array_element _outactors
    (`/Engine/EditorBlueprintResources/StandardMacros.IsValid` _array_element
      (:`Is Valid`
        (set `self.Heavy Base Speed` (`CharacterMovementComponent.MaxWalkSpeed` (`Character.CharacterMovement` _array_element)))
        (break)))))

(event `self.Collision Check X.OnComponentBeginOverlap`
  (params (OverlappedComponent :type "PrimitiveComponent Object Reference") (OtherActor :type "Actor Object Reference") (OtherComp :type "PrimitiveComponent Object Reference") (OtherBodyIndex :type Integer) (bFromSweep :type Boolean) (SweepResult :type "HitResult Structure (by ref)"))
  ;[0 0.05359 1 1 25] Checks if the heavy bot is in bounds to start pushing the object, and enables input to allow for pushing script
)

(event `self.Collision Check Y.OnComponentBeginOverlap`
  (params (OverlappedComponent :type "PrimitiveComponent Object Reference") (OtherActor :type "Actor Object Reference") (OtherComp :type "PrimitiveComponent Object Reference") (OtherBodyIndex :type Integer) (bFromSweep :type Boolean) (SweepResult :type "HitResult Structure (by ref)"))
  ;[0 0.05359 1 1 25] Checks if the heavy bot is in bounds to start pushing the object, and enables input to allow for pushing script
)

(event `self.Collision Check X.OnComponentEndOverlap`
  (params (OverlappedComponent :type "PrimitiveComponent Object Reference") (OtherActor :type "Actor Object Reference") (OtherComp :type "PrimitiveComponent Object Reference") (OtherBodyIndex :type Integer))
  ;[1 0.04843 0.1281 1 25] When the heavy bot leaves these bounds the input is disabled
)

(event `self.Collision Check Y.OnComponentEndOverlap`
  (params (OverlappedComponent :type "PrimitiveComponent Object Reference") (OtherActor :type "Actor Object Reference") (OtherComp :type "PrimitiveComponent Object Reference") (OtherBodyIndex :type Integer))
  ;[1 0.04843 0.1281 1 25] When the heavy bot leaves these bounds the input is disabled
)

(fn `UserConstructionScript`)