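; BP_SoundBox is a trigger volume that plays audio while an Elevator actor passes through its Box.
; On begin overlap, it confirms the Elevator's PlateCollision overlaps it, then reactivates the stored AudioComp or adds one at runtime if none exists.
; On end overlap with an Elevator, it deactivates that component; the plate check there has no effect on the outcome.
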(event `self.Box.OnComponentBeginOverlap`
  (params (OverlappedComponent :type "PrimitiveComponent Object Reference") (OtherActor :type "Actor Object Reference") (OtherComp :type "PrimitiveComponent Object Reference") (OtherBodyIndex :type Integer) (bFromSweep :type Boolean) (SweepResult :type "HitResult Structure (by ref)"))
  (bind _audiocomp (`self.AudioComp`))
  (bind _aselevator (cast `/Game/Blueprint_/JOR_bp/Elevator` OtherActor))
  (if (`PrimitiveComponent.IsOverlappingActor` (`/Game/Blueprint_/JOR_bp/Elevator.Plate Collision` _aselevator) self)
    (`/Engine/EditorBlueprintResources/StandardMacros.IsValid` _audiocomp
      (:`Is Valid`
        (`ActorComponent.Activate` _audiocomp true))
      (:`Is Not Valid`
        (bind _returnvalue (`AddComponent|NODE_AddAudioComponent-0` :`RelativeTransform` (`KismetMathLibrary.Conv_VectorToTransform` (`self.K2_GetActorLocation`))))
        (set `self.AudioComp` _returnvalue)))))

(event `self.Box.OnComponentEndOverlap`
  (params (OverlappedComponent :type "PrimitiveComponent Object Reference") (OtherActor :type "Actor Object Reference") (OtherComp :type "PrimitiveComponent Object Reference") (OtherBodyIndex :type Integer))
  (bind _audiocomp (`self.AudioComp`))
  (bind _aselevator (cast `/Game/Blueprint_/JOR_bp/Elevator` OtherActor))
  (if (`PrimitiveComponent.IsOverlappingActor` (`/Game/Blueprint_/JOR_bp/Elevator.Plate Collision` _aselevator) self)
    _
    (else
      _))
  (`/Engine/EditorBlueprintResources/StandardMacros.IsValid` _audiocomp
    (:`Is Valid`
      (`ActorComponent.Deactivate` _audiocomp))))

(fn `UserConstructionScript`)