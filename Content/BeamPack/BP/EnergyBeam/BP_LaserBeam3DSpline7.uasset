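; Laser beam actor that sweeps via a timeline-driven root rotation and scorches whatever surface it hits.
; The construction script builds spline mesh segments along the spline, keeping the last in NewMesh.
; Each tick traces forward from Point, toggling the LaserBeam and Hit effects on blocking hits.
; Hits align the impact effect, spawn short-lived random-sized fire decals, and stretch spline point 1 and NewMesh to the impact.
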(event `self.ReceiveBeginPlay`
  (bind _defaultsceneroot (`self.DefaultSceneRoot`))
  (bind (_returnvalue_roll _returnvalue_pitch _returnvalue_yaw) (`KismetMathLibrary.BreakRotator` (`SceneComponent.K2_GetComponentRotation` _defaultsceneroot)))
  (bind (_direction _rotex _zrot) (`Timeline|RotateLaser`)
    (:`Update`
      (`SceneComponent.K2_SetWorldRotation` _defaultsceneroot (`KismetMathLibrary.MakeRotator` (* _zrot 20.0) (- _rotex _returnvalue_roll) _returnvalue_yaw) false false))))

(event `self.ReceiveTick`
  (params (DeltaSeconds :type "Float (single-precision)"))
  (bind _returnvalue (`KismetMathLibrary.RandomFloatInRange` 10.0 40.0))
  (bind _returnvalue_2 (`KismetMathLibrary.RandomFloatInRange` 10.0 30.0))
  (bind _point (`self.Point`))
  (bind _spline (`self.Spline`))
  (bind _hit (`self.Hit`))
  (bind _spline_2 (`self.Spline`))
  (bind _returnvalue_3 (`SceneComponent.K2_GetComponentLocation` _point))
  (bind _outhit (`KismetSystemLibrary.LineTraceSingle` _returnvalue_3 (+ _returnvalue_3 (* (`KismetMathLibrary.GetForwardVector` (`SceneComponent.K2_GetComponentRotation` _point)) 3000.0)) "TraceTypeQuery1" true))
  (bind (_bblockinghit _binitialoverlap _time _distance _location _impactpoint _normal) (`GameplayStatics.BreakHitResult` _outhit))
  (if _bblockinghit
    (`ActorComponent.SetActive` (`self.Hit`) true false)
    (`ActorComponent.SetActive` (`self.LaserBeam`) true false)
    (`|ExecutionSequence`
      (:`then_0`
        (bind _returnvalue_4 (`KismetMathLibrary.Conv_VectorToRotator` _normal))
        (`SceneComponent.K2_SetWorldRotation` _hit _returnvalue_4 false false)
        (`SceneComponent.K2_SetWorldLocation` _hit (+ _location 10) false false)
        (`GameplayStatics.SpawnDecalAtLocation` "/Game/BeamPack/Materials/M_FireDecal.M_FireDecal" (`KismetMathLibrary.MakeVector` _returnvalue _returnvalue _returnvalue) _location _returnvalue_4 5.0)
        (`GameplayStatics.SpawnDecalAtLocation` "/Game/BeamPack/Materials/Instance/MI_Fire_DecalGoldern.MI_Fire_DecalGoldern" (`KismetMathLibrary.MakeVector` _returnvalue_2 _returnvalue_2 _returnvalue_2) _location _returnvalue_4 3.0))
      (:`then_1`
        (`SplineComponent.SetLocationAtSplinePoint` (`self.Spline`) 1 _location "World" true)
        (`SplineMeshComponent.SetStartAndEnd` (`self.NewMesh`) (`SplineComponent.GetLocationAtSplinePoint` _spline 0 "Local") (`SplineComponent.GetTangentAtSplinePoint` _spline 0 "Local") (`SplineComponent.GetLocationAtSplinePoint` _spline_2 1 "Local") (`SplineComponent.GetTangentAtSplinePoint` _spline_2 1 "Local") true)))
    (else
      (`ActorComponent.SetActive` (`self.Hit`) false false)
      (`ActorComponent.SetActive` (`self.LaserBeam`) false false))))

(fn `UserConstructionScript`
  (bind _spline (`self.Spline`))
  (bind _spline_2 (`self.Spline`))
  (for _index (range (+ (- (`SplineComponent.GetNumberOfSplinePoints` (`self.Spline`)) 2) 1))
    (bind _returnvalue (`AddComponent|NODE_AddSplineMeshComponent-0`))
    (bind _output_get (set `self.NewMesh` _returnvalue))
    (`SplineMeshComponent.SetForwardAxis` _output_get "Z" true)
    (bind _returnvalue_2 (+ _index 1))
    (`SplineMeshComponent.SetStartAndEnd` _output_get (`SplineComponent.GetLocationAtSplinePoint` _spline _index "Local") (`SplineComponent.GetTangentAtSplinePoint` _spline 0 "Local") (`SplineComponent.GetLocationAtSplinePoint` _spline_2 _returnvalue_2 "Local") (`SplineComponent.GetTangentAtSplinePoint` _spline_2 _returnvalue_2 "Local") true)))