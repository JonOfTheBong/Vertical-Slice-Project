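; Laser beam effect actor that sweeps its pitch through a downward arc with the RotateLaser timeline started on BeginPlay.
; Each Tick, a visibility line trace from Point sets the LaserBeam Niagara mesh scale from the distance to the hit.
; The Hit component follows the impact location with a small offset and aligns to the surface normal.
; Delayed, randomly sized fire decal spawning at the impact is present but never runs.
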(event `self.ReceiveBeginPlay`
  (bind (_direction _rotex) (`Timeline|RotateLaser`)
    (:`Update`
      (`SceneComponent.K2_SetWorldRotation` (`self.DefaultSceneRoot`) (`KismetMathLibrary.MakeRotator` 0.0 (`KismetMathLibrary.Lerp` -60.0 -120.0 _rotex)) false false))))

(event `self.ReceiveTick`
  (params (DeltaSeconds :type "Float (single-precision)"))
  (bind _point (`self.Point`))
  (bind _hit (`self.Hit`))
  (bind _returnvalue (`SceneComponent.K2_GetComponentLocation` _point))
  (bind _outhit (`KismetSystemLibrary.LineTraceSingle` _returnvalue (+ _returnvalue (* (`KismetMathLibrary.GetForwardVector` (`SceneComponent.K2_GetComponentRotation` _point)) 1500.0)) "TraceTypeQuery1" true))
  (bind (_bblockinghit _binitialoverlap _time _distance _location _impactpoint _normal) (`GameplayStatics.BreakHitResult` _outhit))
  (`NiagaraComponent.SetVariableFloat` (`self.LaserBeam`) "User.Z_Mesh Scale" (/ (`KismetMathLibrary.Vector_Distance` (`SceneComponent.K2_GetComponentLocation` (`self.Point`)) _location) 12.0))
  (`SceneComponent.K2_SetWorldRotation` _hit (`KismetMathLibrary.Conv_VectorToRotator` _normal) false false)
  (`SceneComponent.K2_SetWorldLocation` _hit (+ _location 10) false false))

(fn `UserConstructionScript`)