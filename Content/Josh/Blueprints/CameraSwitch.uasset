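; Camera switch trigger volume that changes the Main character's active camera while it is inside the Box.
; Begin overlap activates Camera over FollowCamera, and end overlap restores FollowCamera.
; Each switch waits briefly, then snaps the player's control rotation to a fixed yaw.
; Paired DoOnce gates re-arm each other to alternate switches; disconnected camera offset and boom nodes never run.
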(event `self.Box.OnComponentBeginOverlap`
  (params (OverlappedComponent :type "PrimitiveComponent Object Reference") (OtherActor :type "Actor Object Reference") (OtherComp :type "PrimitiveComponent Object Reference") (OtherBodyIndex :type Integer) (bFromSweep :type Boolean) (SweepResult :type "HitResult Structure (by ref)"))
  (bind _asmain (cast `/Game/ThirdPersonBP/Blueprints/Main` OtherActor))
  (`/Engine/EditorBlueprintResources/StandardMacros.DoOnce` false :!label _label
    (:`Completed`
      (`ActorComponent.SetActive` (`/Game/ThirdPersonBP/Blueprints/Main.FollowCamera` _asmain) false false)
      (`ActorComponent.SetActive` (`/Game/ThirdPersonBP/Blueprints/Main.Camera` _asmain) true false)
      (`KismetSystemLibrary.Delay` 1.0)
      (`Controller.SetControlRotation` (`GameplayStatics.GetPlayerController` 0) (`KismetMathLibrary.MakeRotator` 0.0 0.0 270.0))
      (goto _label_2 :!via `Reset`))))

(event `self.Box.OnComponentEndOverlap`
  (params (OverlappedComponent :type "PrimitiveComponent Object Reference") (OtherActor :type "Actor Object Reference") (OtherComp :type "PrimitiveComponent Object Reference") (OtherBodyIndex :type Integer))
  (bind _asmain (cast `/Game/ThirdPersonBP/Blueprints/Main` OtherActor))
  (`/Engine/EditorBlueprintResources/StandardMacros.DoOnce` false :!label _label_2
    (:`Completed`
      (`ActorComponent.SetActive` (`/Game/ThirdPersonBP/Blueprints/Main.Camera` _asmain) false false)
      (`ActorComponent.SetActive` (`/Game/ThirdPersonBP/Blueprints/Main.FollowCamera` _asmain) true false)
      (`KismetSystemLibrary.Delay` 1.0)
      (`Controller.SetControlRotation` (`GameplayStatics.GetPlayerController` 0) (`KismetMathLibrary.MakeRotator` 0.0))
      (goto _label :!via `Reset`))))

(fn `UserConstructionScript`)