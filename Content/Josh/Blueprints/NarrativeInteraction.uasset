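; Interactable narrative trigger actor that shows a text screen when a Main or Heavy character stands in its Box and presses Interact.
; On overlap it enables input, reveals a prompt widget, creates a NarrativeInteractionWidget filled with its NarrativeText and opens a gate.
; The Interact press passes through the gate to add that widget to the viewport.
; Leaving the box disables input, hides the prompt and removes the text widget from the screen.
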(event `InputAction|Interact`
  (params (Key :type "Key Structure"))
  (:`Pressed`
    (`/Engine/EditorBlueprintResources/StandardMacros.Gate` true :!label _label
      (:`Exit`
        (`UserWidget.AddToViewport` (stale `self.Box.OnComponentBeginOverlap` _returnvalue) 0)))))

(event `self.Box.OnComponentBeginOverlap`
  (params (OverlappedComponent :type "PrimitiveComponent Object Reference") (OtherActor :type "Actor Object Reference") (OtherComp :type "PrimitiveComponent Object Reference") (OtherBodyIndex :type Integer) (bFromSweep :type Boolean) (SweepResult :type "HitResult Structure (by ref)"))
  ;[1 1 1] Creates widget
  (cast `/Game/ThirdPersonBP/Blueprints/Main` OtherActor
    (:`then`
      _)
    (:`CastFailed`
      (cast `/Game/ThirdPersonBP/Blueprints/Heavy` OtherActor)))
  (`self.EnableInput` (`GameplayStatics.GetPlayerController` 0))
  (`SceneComponent.SetHiddenInGame` (`self.Widget`) false false)
  ;[1 1 1] Adds widget to viewport when "E" is pressed
  (bind _returnvalue (`|CreateWidget` "/Game/Josh/Blueprints/NarrativeInteractionWidget.NarrativeInteractionWidget_C"))
  (set `/Game/Josh/Blueprints/NarrativeInteractionWidget.NarrativeText` (`self.NarrativeText`) _returnvalue)
  (goto _label :!via `Open`))

(event `self.Box.OnComponentEndOverlap`
  (params (OverlappedComponent :type "PrimitiveComponent Object Reference") (OtherActor :type "Actor Object Reference") (OtherComp :type "PrimitiveComponent Object Reference") (OtherBodyIndex :type Integer))
  ;[1 1 1] Checks for player overlap, if no overlap sets "has left area" to true, removes parent = removing text from screen.
  (cast `/Game/ThirdPersonBP/Blueprints/Main` OtherActor
    (:`then`
      _)
    (:`CastFailed`
      (cast `/Game/ThirdPersonBP/Blueprints/Heavy` OtherActor)))
  (`self.DisableInput` (`GameplayStatics.GetPlayerController` 0))
  (`SceneComponent.SetHiddenInGame` (`self.Widget`) true false)
  (set `self.HasLeftArea` true)
  (if (`self.HasLeftArea`)
    (`Widget.RemoveFromParent` (stale `self.Box.OnComponentBeginOverlap` _returnvalue))
    (`KismetSystemLibrary.PrintString` "screen removed")))

(fn `UserConstructionScript`)